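; BP_Camera is a side-on 2D camera actor that tracks the player character and frames it with an active grapple target.
; BeginPlay caches the player, while UpdateCamera and ClearCamera set or drop the current grapple.
; With a grapple, Tick eases toward a weighted Y/Z point derived from both positions, keeping depth.
; Otherwise it snaps to the player at a fixed X follow distance.
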(event `self.ReceiveBeginPlay`
  (bind _asbp_character_base_2d (cast `/Game/Blueprints/BP_CharacterBase2D` (`GameplayStatics.GetPlayerCharacter` 0))
    (:`then`
      (`self.SetupCamera` _asbp_character_base_2d))
    (:`CastFailed`
      (`KismetSystemLibrary.PrintString` "Failed to find Player"))))

(event `self.ReceiveTick`
  (params (DeltaSeconds :type "Float (single-precision)"))
  (bind _returnvalue (`self.K2_GetActorLocation`))
  (bind _player (`self.Player`))
  (bind _current_grapple (`self.Current Grapple`))
  (bind (_x _y _z) (`KismetMathLibrary.BreakVector3f` (`self.K2_GetActorLocation` _player)))
  (bind (_x_2 _y_2 _z_2) (`KismetMathLibrary.BreakVector3f` (`self.K2_GetActorLocation` _current_grapple)))
  (if (and (`KismetSystemLibrary.IsValid` _player) (`KismetSystemLibrary.IsValid` _current_grapple))
    (`self.K2_SetActorLocation` (`KismetMathLibrary.VLerp` _returnvalue (`KismetMathLibrary.MakeVector` (`KismetMathLibrary.BreakVector3f` _returnvalue) (/ (+ _y _y_2) 2.0) (/ (+ _z _z_2) 1.2)) (* (`GameplayStatics.GetWorldDeltaSeconds`) 1.2)) true)
    (else
      (`self.Follow Player` (`self.Follow Distance`)))))

(fn `Clear Camera`
  (set `self.Current Grapple` null))

(fn `Follow Player`
  (params (`Camera Boom` :type "Float (double-precision)"))
  (bind (_x _y _z) (`KismetMathLibrary.BreakVector3f` (`self.K2_GetActorLocation` (`self.Player`))))
  (`/Engine/EditorBlueprintResources/StandardMacros.IsValid` (`self.Player`)
    (:`Is Valid`
      (`self.K2_SetActorLocation` (`KismetMathLibrary.MakeVector` `Camera Boom` _y _z)))))

(fn `Setup Player Only Camera`)

(fn `SetupCamera`
  (params (Player :type "/Game/Blueprints/BP_CharacterBase2D Object Reference"))
  (`/Engine/EditorBlueprintResources/StandardMacros.IsValid` Player
    (:`Is Valid`
      (set `self.Player` Player))))

(fn `Update Camera`
  (params (`New Grapple` :type "/Game/Blueprints/BP_GrapplePawn Object Reference"))
  (`/Engine/EditorBlueprintResources/StandardMacros.IsValid` `New Grapple`
    (:`Is Valid`
      (set `self.Current Grapple` `New Grapple`))))

(fn `UserConstructionScript`)