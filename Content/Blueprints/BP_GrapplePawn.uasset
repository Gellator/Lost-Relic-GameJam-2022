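; Pawn for a grapple point that aims with the mouse and fires to place further grapple points, forming a chain.
; Aim intersects the mouse ray with the plane at the pawn's X, giving side-on aiming from its Cube.
; Fire traces toward that point, spawns a linked BP_GrapplePawn on static mesh actor hits and sets it as the Player's CurrentGrapple.
; T returns possession to the Player; grapple length is only stored here.
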(event `Key|T`
  (params (Key :type "Key Structure"))
  (bind _player (`self.Player`))
  (:`Pressed`
    (if (`self.isActive`)
      _
      (else
        _))
    (`KismetSystemLibrary.PrintString` (`KismetSystemLibrary.GetDisplayName` _player))
    (`Controller.Possess` (`GameplayStatics.GetPlayerController` 0) _player)
    (`KismetSystemLibrary.PrintString` "Posses character")))

(event `InputAxis|Aim`
  (params (AxisValue :type "Float (single-precision)"))
  (`self.Aimstyle 2`))

(event `Aimstyle 2`
  (bind (_worldlocation _worlddirection) (`PlayerController.DeprojectMousePositionToWorld` (`GameplayStatics.GetPlayerController` 0)))
  (bind _returnvalue (+ _worldlocation (* _worlddirection 100000.0)))
  (`KismetSystemLibrary.LineTraceSingle` _worldlocation _returnvalue "TraceTypeQuery1")
  (bind _location (`self.Aim test` _worldlocation _returnvalue))
  (set `self.Aim Location` _location)
  (`KismetSystemLibrary.LineTraceSingle` :`Start` (`SceneComponent.K2_GetComponentLocation` (`self.Cube`)) :`End` _location :`TraceChannel` "TraceTypeQuery1" :`DrawDebugType` "ForOneFrame"))

(event `InputAction|Fire`
  (params (Key :type "Key Structure"))
  (bind _player (`self.Player`))
  (:`Pressed`
    (bind (_outhit _returnvalue) (`KismetSystemLibrary.LineTraceSingle` (`SceneComponent.K2_GetComponentLocation` (`self.Cube`)) (`self.Aim Location`) "TraceTypeQuery1"))
    (if _returnvalue
      (bind (_bblockinghit _binitialoverlap _time _distance _location _impactpoint _normal _impactnormal _physmat _hitactor) (`GameplayStatics.BreakHitResult` _outhit))
      (cast `StaticMeshActor` _hitactor)
      (bind (_x _y _z) (`KismetMathLibrary.BreakVector3f` _location))
      (bind _returnvalue_2 (`|SpawnActorFromClass` "BP_GrapplePawn_C" (`KismetMathLibrary.MakeTransform` (`KismetMathLibrary.MakeVector` _x _y _z)) "AdjustIfPossibleButAlwaysSpawn" "OverrideRootScale" null null))
      (`self.Setup Grapple` _returnvalue_2 self 100.0 _player)
      (set `/Game/Blueprints/BP_CharacterBase2D.Current Grapple` _returnvalue_2 _player))))

(fn `Aim test`
  (params (Start :type "Vector Structure") (Target :type "Vector Structure"))
  (returns (Location :type "Vector Structure"))
  (bind _returnvalue_x (`KismetMathLibrary.BreakVector` (`self.K2_GetActorLocation`)))
  (bind (_x _y _z) (`KismetMathLibrary.BreakVector3f` Start))
  (bind (_x_2 _y_2 _z_2) (`KismetMathLibrary.BreakVector3f` Target))
  (return (`KismetMathLibrary.MakeVector` _returnvalue_x (+ (/ (* (- _returnvalue_x _x) (- _y_2 _y)) (- _x_2 _x)) _y) (+ _z (/ (* (- _returnvalue_x _x) (- _z_2 _z)) (- _x_2 _x))))))

(fn `Setup Grapple`
  (params (`Previous Grapple` :type "/Game/Blueprints/BP_GrapplePawn Object Reference") (`Grapple Length` :type "Float (double-precision)") (Player :type "/Game/Blueprints/BP_CharacterBase2D Object Reference"))
  (set `self.isActive` true)
  (set `self.Previous Grapple` `Previous Grapple`)
  (set `self.Grapple Length` `Grapple Length`)
  (set `self.Player` Player))

(fn `UserConstructionScript`)